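; Light Blueprint that wraps a SpotLight and lets it be switched on and off.
; ToggleLights flips the IsOn flag, applies it to the spotlight's visibility and sets the light color from the NewLightColor variable.
; The construction script applies IsOn to visibility, so the initial on/off state shows at placement.
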(event EventToggleLights
  (bind _output_get (Variables|Default|SetIs%20on (not (Variables|Default|GetIs%20on))))
  (Rendering|SetVisibility (Variables|Default|GetSpotLight) _output_get false)
  (Rendering|Components|Light|SetLightColor (Variables|Default|GetSpotLight) (Variables|Default|GetNew%20Light%20Color) true))

(fn ConstructionScript
  (Rendering|SetVisibility (Variables|Default|GetSpotLight) (Variables|Default|GetIs%20on) false))